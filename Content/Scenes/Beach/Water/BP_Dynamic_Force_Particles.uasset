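; Water force actor for the beach scene that emits Niagara splash particles when it enters or leaves a WaterBodyOcean.
; On BeginPlay it sizes its collision sphere and splash effect from the force radius.
; Tick records per-frame movement, which EmitSplash uses to set particle direction, with Z forced upward, and to scale particle count with speed before restarting the effect.
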(event Collision|EventActorBeginOverlap
  (params (OtherActor :type Actor%20Object%20Reference))
  ;[1 1 1] Splash particles
  (if (Utilities|ClassIsChildOf (Utilities|GetClass OtherActor) "/Script/Water.WaterBodyOcean")
    (CallFunction|EmitSplash (Variables|Default|GetLocationChange))))

(event EventBeginPlay
  (bind _radius (Variables|Default|GetRadius))
  (|CallParentFunction)
  ;[1 1 1] Set collision and splash radius to ForceMesh radius on start
  (Components|Sphere|SetSphereRadius (Variables|Default|GetSphere) _radius true)
  (Effects|Components|ParticleSystem|SetFloatParameter (Variables|Default|GetNS_Splash) "SplashRadius" _radius)
  (Variables|Default|SetPreviousLocation (Transformation|GetWorldLocation (Variables|Default|GetDefaultSceneRoot))))

(event EventTick
  (params (DeltaSeconds :type Float%20%28single-precision%29))
  (bind _defaultsceneroot (Variables|Default|GetDefaultSceneRoot))
  (bind _returnvalue (Transformation|GetWorldLocation _defaultsceneroot))
  (|CallParentFunction DeltaSeconds)
  ;[1 1 1] Update LocationChange
  (Variables|Default|SetLocationChange (- _returnvalue (Variables|Default|GetPreviousLocation)))
  (Variables|Default|SetPreviousLocation _returnvalue))

(event Collision|EventActorEndOverlap
  (params (OtherActor :type Actor%20Object%20Reference))
  ;[1 1 1] Splash particles
  (if (Utilities|ClassIsChildOf (Utilities|GetClass OtherActor) "/Script/Water.WaterBodyOcean")
    (CallFunction|EmitSplash (Variables|Default|GetLocationChange))))

(fn ConstructionScript
  (|CallParentFunction))

(fn EmitSplash
  (params (Speed :type Vector))
  (bind (_x _y _z) (Class|KismetMathLibrary|BreakVector3f Speed))
  (bind _ns_splash (Variables|Default|GetNS_Splash))
  ;[1 1 1] Particle direction
  (Effects|Components|ParticleSystem|SetVectorParameter _ns_splash "Direction" (Math|Vector|MakeVector _x _y (Math|Float|Absolute(Float) _z)))
  ;[1 1 1] Particle amount depending on speed
  (Effects|Components|ParticleSystem|SetIntParameter _ns_splash "ParticleAmount" (Math|Float|Truncate (* (Math|Vector|VectorLength Speed) 5e+01)))
  (Components|Activation|SetActive _ns_splash true true))